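; Throwable USMC grenade projectile that bounces, counts down a fuse on Tick and applies explosive damage when it detonates.
; Hits play physical-material impact effects, falling back to surface-selected bounce sounds with speed-scaled volume.
; Overlapping flagged physical materials disables bouncing and stores the hit for an extra explosion effect.
; Explosion cosmetics are gated, with a legacy emitter, sound and shockwave fallback when no material effect plays.
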(event `self.CollisionComp.OnComponentBeginOverlap`
  (params (OverlappedComponent :type "PrimitiveComponent Object Reference") (OtherActor :type "Actor Object Reference") (OtherComp :type "PrimitiveComponent Object Reference") (OtherBodyIndex :type Integer) (bFromSweep :type Boolean) (SweepResult :type "HitResult Structure (by ref)"))
  (bind _assqphysical_material (cast `SQPhysicalMaterial` (`.PhysMat` (`GameplayStatics.BreakHitResult` SweepResult))))
  (if (`SQPhysicalMaterial.bOverlapsThrowableProjectiles` _assqphysical_material)
    (set `ProjectileMovementComponent.bShouldBounce` false (`self.ProjectileMovement`))
    (`/Engine/EditorBlueprintResources/StandardMacros.Can Execute Cosmetic Events`
      (:`True`
        (`self.PlayThrowableImpactEffect` SweepResult)
        (set `self.Last Overlap Hit Result` SweepResult)
        (set `self.bOverlapOccurred` true)))))

(event `self.ReceiveTick`
  (params (DeltaSeconds :type "Float (single-precision)"))
  (if (and (< (`self.FuseTime`) 0.0) (not (`self.bIsExploding`)) (`self.bExplodeOnFuse`))
    (`self.Explode`)
    (set `self.bIsExploding` true)
    (else
      (set `self.FuseTime` (- (`self.FuseTime`) DeltaSeconds)))))

(event `self.ReceiveHit`
  (params (MyComp :type "PrimitiveComponent Object Reference") (Other :type "Actor Object Reference") (OtherComp :type "PrimitiveComponent Object Reference") (bSelfMoved :type Boolean) (HitLocation :type "Vector Structure") (HitNormal :type "Vector Structure") (NormalImpulse :type "Vector Structure") (Hit :type "HitResult Structure (by ref)"))
  (bind (_bblockinghit _binitialoverlap _time _location _impactpoint _normal _impactnormal _physmat) (`GameplayStatics.BreakHitResult` Hit))
  (bind _dirtbouncesound (`self.DirtBounceSound`))
  (bind _returnvalue (`KismetMathLibrary.VSize` (`self.GetVelocity`)))
  (bind _returnvalue_2 (select `EPhysicalSurface` (`PhysicalMaterial.SurfaceType` _physmat) :`SurfaceType_Default` _dirtbouncesound :`SurfaceType1` (`self.ConcreteBounceSound`) :`SurfaceType2` _dirtbouncesound :`SurfaceType4` (`self.MetalBounceSound`) :`SurfaceType5` (`self.WoodBounceSound`) :`SurfaceType6` _dirtbouncesound :`SurfaceType7` _dirtbouncesound :`SurfaceType8` _dirtbouncesound :`SurfaceType9` _dirtbouncesound :!type "SoundBase Object Reference"))
  (set `self.bHasImpacted` true)
  (bind _returnvalue_3 (`self.PlayThrowableImpactEffect` Hit))
  (if (not _returnvalue_3)
    (`/Engine/EditorBlueprintResources/StandardMacros.Can Execute Cosmetic Events`
      (:`True`
        (if (> _returnvalue 100.0)
          (`/Engine/EditorBlueprintResources/StandardMacros.IsValid` _returnvalue_2
            (:`Is Valid`
              (`GameplayStatics.PlaySoundAtLocation` _returnvalue_2 (+ _location _impactnormal) (struct) (`KismetMathLibrary.FMin` (/ _returnvalue 1500.0) 1.5)))))))))

(fn `Explode`
  (set `self.bIsExploding` true)
  (`self.BPApplyExplosiveDamage` (`self.LastImpactHitResult`) (`self.GetWeapon` self) (`|MakeArray` self :!type "Actor Object Reference"))
  (`PrimitiveComponent.SetCollisionEnabled` (`self.CollisionComp`) "NoCollision")
  (`/Engine/EditorBlueprintResources/StandardMacros.Can Execute Cosmetic Events`
    (:`True`
      (`SceneComponent.SetVisibility` (`self.SkeletalMesh`) false true)
      (`|ExecutionSequence`
        (:`then_0`
          (bind _returnvalue (`self.PlayExplosionEffect` (`self.LastImpactHitResult`)))
          (if (not _returnvalue)
            ;[1 1 1] For backwards compatibility or if some physical materials are not st up properly for explosion effects
            (`self.SpawnEmitter`)
            (`GameplayStatics.PlaySoundAtLocation` (`self.ExplosionSound`) (`self.K2_GetActorLocation`))
            (bind _asbp_shockwave (cast `/Game/Blueprints/Effects/BP_Shockwave` (`ChildActorComponent.ChildActor` (`self.Shockwave`))))
            (`/Game/Blueprints/Effects/BP_Shockwave.Explode` _asbp_shockwave (`self.Instigator`))))
        (:`then_1`
          (if (`self.bOverlapOccurred`)
            (`self.PlayExplosionEffect` (`self.Last Overlap Hit Result`))))))))

(fn `SpawnEmitter`
  (`GameplayStatics.SpawnEmitterAtLocation` (`self.ExplosionEffect`) (`self.K2_GetActorLocation`)))

(fn `UserConstructionScript`)